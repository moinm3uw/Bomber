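; Game instance that sets up online multiplayer sessions and handles session invites for Bomber.
; Outside the editor, Init waits briefly, then creates an advanced session unless "nosteam" is on the command line, reopening the current level as a listen server on success.
; Both received and accepted invites destroy any current session and join automatically, even if destruction fails.
; A successful join hides all widgets and switches the view to a tagged black-view camera as loading screen.
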(event `self.ReceiveInit`
  (`KismetSystemLibrary.Delay` 0.5)
  (if (not (`UtilsLibrary.IsEditor`))
    (bind _returnvalue (`KismetSystemLibrary.GetCommandLine`))
    (if (not (`KismetStringLibrary.Contains` _returnvalue "nosteam"))
      (`self.CreateAdvancedSession`)
      (else
        (`KismetSystemLibrary.PrintString` "NOSTEAM" true true (struct :`R` 1.0 :`G` 0.00746 :`A` 1.0) 10.0)))))

(event `CreateAdvancedSession`
  (bind _returnvalue (`MyBlueprintFunctionLibrary.GetLocalPlayerController`))
  (`/Engine/EditorBlueprintResources/StandardMacros.IsValid` _returnvalue
    (:`Is Valid`
      (`KismetSystemLibrary.PrintString` "Attempt")
      (`CreateSessionCallbackProxyAdvanced.CreateAdvancedSession` :`PlayerController` _returnvalue
        (:`OnSuccess`
          (`KismetSystemLibrary.PrintString` "Session Created!" true true (struct :`R` 0.023588 :`G` 1.0 :`A` 1.0) 10.0)
          (`self.ReopenLevelAsListen`))
        (:`OnFailure`
          (`KismetSystemLibrary.PrintString` "Failed to create session!" true true (struct :`R` 1.0 :`G` 0.00746 :`A` 1.0) 10.0))))
    (:`Is Not Valid`
      (`KismetSystemLibrary.PrintString` "EMPTY CONTROLLER" true true (struct :`R` 1.0 :`G` 0.00746 :`A` 1.0) 10.0))))

(event `ReopenLevelAsListen`
  (bind _returnvalue (`GameplayStatics.GetCurrentLevelName` true))
  (`GameplayStatics.OpenLevel` (`KismetStringLibrary.Conv_StringToName` _returnvalue) true "listen"))

(event `self.OnSessionInviteAccepted`
  (params (LocalPlayerNum :type Integer) (PersonInvited :type "BPUniqueNetId Structure") (SessionToJoin :type "BlueprintSessionResult Structure (by ref)"))
  (bind _returnvalue (`GameplayStatics.GetPlayerController` 0))
  (`DestroySessionCallbackProxy.DestroySession` _returnvalue
    (:`OnSuccess`
      _)
    (:`OnFailure`
      _))
  (`KismetSystemLibrary.PrintString` "Invite Accepted, joining session")
  (`JoinSessionCallbackProxy.JoinSession` _returnvalue SessionToJoin
    (:`OnSuccess`
      (`KismetSystemLibrary.PrintString` "Joining session!")
      (`self.DisplayLoadingScreen`))
    (:`OnFailure`
      (`KismetSystemLibrary.PrintString` "Failed to join session"))))

(event `self.OnSessionInviteReceived`
  (params (LocalPlayerNum :type Integer) (PersonInviting :type "BPUniqueNetId Structure") (AppId :type String) (SessionToJoin :type "BlueprintSessionResult Structure (by ref)"))
  (bind _returnvalue (`GameplayStatics.GetPlayerController` 0))
  (`DestroySessionCallbackProxy.DestroySession` _returnvalue
    (:`OnSuccess`
      _)
    (:`OnFailure`
      _))
  (`KismetSystemLibrary.PrintString` "Invite Received, joining session")
  (`JoinSessionCallbackProxy.JoinSession` _returnvalue SessionToJoin
    (:`OnSuccess`
      (`KismetSystemLibrary.PrintString` "Joining session!")
      (`self.DisplayLoadingScreen`))
    (:`OnFailure`
      (`KismetSystemLibrary.PrintString` "Failed to join session"))))

(event `DisplayLoadingScreen`
  (bind _outactors (`GameplayStatics.GetAllActorsWithTag` "StartupBlackViewCamera"))
  (`PlayerController.SetViewTargetWithBlend` (`MyBlueprintFunctionLibrary.GetLocalPlayerController`) (`|GetArrayItem` _outactors) 0.0 "VTBlend_Linear" 0.0 false)
  (`WidgetsSubsystem.SetAllWidgetsVisibility` (`WidgetsSubsystem.GetWidgetsSubsystem`) false))